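; Paintable static mesh actor that receives brush strokes on a Basecolor map through its BCPaintSystem component.
; Construction hooks a SceneCaptureComponent2D into the paint system, and BeginPlay or SetupMeshes registers the mesh with that map.
; Paint forwards directional strokes with tint and shape, falling back to a default grid texture when no brush is valid.
; SetStaticMesh swaps the mesh without re-running setup.
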(event Custom|Paint
  (params (Location :type Vector) (Normal :type Vector) (Rotation :type Float%20%28single-precision%29) (Size :type Float%20%28single-precision%29) (Opacity :type Float%20%28double-precision%29) (Brush :type Texture%20Object%20Reference) (BrushTint :type Linear%20Color%20Structure :default "(R=1.000000,G=1.000000,B=1.000000,A=1.000000)") (BrushShape :type E_PaintBrushShapeType%20Enum :default "NewEnumerator0"))
  (bind _output_get (Variables|Default|SetBrush Brush))
  (Utilities|IsValid _output_get
    (:Is%20Valid
      _)
    (:Is%20Not%20Valid
      (Variables|Default|SetBrush "/Engine/EngineMaterials/DefaultWhiteGrid_Low.DefaultWhiteGrid_Low")))
  (Default|PaintwithDirection (Variables|Default|GetBC_PaintSystem) "Basecolor" Location Normal "None" Rotation Size Opacity (Variables|Default|GetBrush) BrushShape 1e+01 BrushTint))

(event Custom|SetStaticMesh
  (params (NewMesh :type Static%20Mesh%20Object%20Reference))
  (Utilities|IsValid NewMesh
    (:Is%20Valid
      (Components|StaticMesh|SetStaticMesh (Variables|Default|GetPaintStaticMesh) NewMesh))))

(event Custom|SetupMeshes
  (Default|SetupMeshes (Variables|Default|GetBC_PaintSystem) (Utilities|Array|MakeArray (Utilities|Struct|MakeBST_PaintSetupData (Variables|Default|GetPaintStaticMesh) 0 0 "0.000000,0.000000,0.000000" (Utilities|Array|MakeArray (Utilities|Struct|MakeBST_PaintMapData "Basecolor" "NewEnumerator0" (Variables|Default|GetSize)))))))

(event EventBeginPlay
  (Default|SetupMeshes (Variables|Default|GetBC_PaintSystem) (Utilities|Array|MakeArray (Utilities|Struct|MakeBST_PaintSetupData (Variables|Default|GetPaintStaticMesh) 0 0 "0.000000,0.000000,0.000000" (Utilities|Array|MakeArray (Utilities|Struct|MakeBST_PaintMapData "Basecolor" "NewEnumerator0" (Variables|Default|GetSize)))))))

(fn ConstructionScript
  (Default|SetupSceneCapture (Variables|Default|GetBC_PaintSystem) (Variables|Default|GetSceneCaptureComponent2D) true))